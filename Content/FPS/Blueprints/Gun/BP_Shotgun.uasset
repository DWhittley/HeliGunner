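; BP_Shotgun is a child gun Blueprint for the shotgun weapon, overriding the parent's Shoot function.
; Shoot calls the parent, then runs a single Visibility line trace between the supplied start and end positions and applies Damage to the hit actor.
; The trace has no pellet spread and briefly draws debug lines; the event graph holds only disabled default events.
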(fn `Shoot`
  (params (`Start Position` :type "Vector Structure") (`End Position` :type "Vector Structure"))
  (`parent.Shoot` `Start Position` `End Position`)
  (bind _outhit (`KismetSystemLibrary.LineTraceSingle` :`Start` `Start Position` :`End` `End Position` :`TraceChannel` "TraceTypeQuery1" :`DrawDebugType` "ForDuration" :`DrawTime` 0.1))
  (`GameplayStatics.ApplyDamage` (`.HitActor` (`GameplayStatics.BreakHitResult` _outhit)) (`self.Damage`)))

(fn `UserConstructionScript`
  (`parent.UserConstructionScript`))