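; BP_Rifle is a hitscan rifle Blueprint that extends a parent gun class's Shoot and tracks its own ammo use.
; Shoot calls the parent, then, if ammo remains, line-traces on Visibility with a brief debug line and spends one round.
; It attaches a temporary bullet-hole decal at the impact and applies Damage to the hit actor, without checking for a hit.
; The AddAmmo event increases the ammo count.
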(event `AddAmmo`
  (params (AmmoAmount :type Integer))
  (set `self.Ammo` (+ AmmoAmount (`self.Ammo`))))

(fn `NewFunction`)

(fn `Shoot`
  (params (`Start Position` :type "Vector Structure") (`End Position` :type "Vector Structure"))
  (`parent.Shoot` `Start Position` `End Position`)
  (if (> (`self.Ammo`) 0)
    (bind _outhit (`KismetSystemLibrary.LineTraceSingle` :`Start` `Start Position` :`End` `End Position` :`TraceChannel` "TraceTypeQuery1" :`DrawDebugType` "ForDuration" :`TraceHitColor` (struct :`R` 1.0 :`G` 0.048188 :`A` 1.0) :`DrawTime` 0.1))
    ;[1 1 1] Reduce ammo by 1
    (set `self.Ammo` (- (`self.Ammo`) 1))
    (bind (_bblockinghit _binitialoverlap _time _distance _location _impactpoint _normal _impactnormal _physmat _hitactor _hitcomponent) (`GameplayStatics.BreakHitResult` _outhit))
    ;[1 1 1] Apply bullet hole
    (`GameplayStatics.SpawnDecalAttached` "/Game/FPS/Textures/T_BulletHole.T_BulletHole" (5.0 10.0 10.0) _hitcomponent "None" _impactpoint (`KismetMathLibrary.Conv_VectorToRotator` _impactnormal) "KeepWorldPosition" 10.0)
    (`GameplayStatics.ApplyDamage` _hitactor (`self.Damage`))))

(fn `UserConstructionScript`)