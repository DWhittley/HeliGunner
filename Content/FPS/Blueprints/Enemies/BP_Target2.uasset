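; BP_Target2 is a child target Blueprint in the FPS enemy set that awards score when it takes damage.
; TakeDamage runs the parent logic, then adds its AddScorePoints value to the score through GM_FPSMap.
; CustomDestroy extends the parent by setting the Sphere's visibility, but derives the Sphere's collision from remaining health in BPHealthComponent rather than the HasCollision input.
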(fn `CustomDestroy`
  (params (isVisible :type Boolean) (HasCollision :type Boolean))
  (bind _sphere (`self.Sphere`))
  (`parent.CustomDestroy` isVisible HasCollision)
  (`SceneComponent.SetVisibility` (`self.Sphere`) isVisible false)
  (if (> (`/Game/FPS/Blueprints/BP_Health_Component.Health` (`self.BP_Health_Component`)) 0.0)
    (`PrimitiveComponent.SetCollisionEnabled` _sphere "QueryAndPhysics")
    (else
      (`PrimitiveComponent.SetCollisionEnabled` _sphere "NoCollision"))))

(fn `NewFunction_0`)

(fn `TakeDamage`
  (params (Damage :type "Float (double-precision)"))
  (`parent.TakeDamage` Damage)
  (bind _asgm_fpsmap (cast `/Game/FPS/Blueprints/GM_FPSMap` (`GameplayStatics.GetGameMode`)))
  (`/Game/FPS/Blueprints/GM_FPSMap.AddPointsToScore` _asgm_fpsmap (`self.Add Score Points`)))

(fn `UserConstructionScript`
  (`parent.UserConstructionScript`))