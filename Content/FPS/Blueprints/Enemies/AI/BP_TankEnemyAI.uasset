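; Tank enemy for the FPS mode, extending parent damage, destroy and attack behaviour.
; Taking damage grows a fire Niagara effect as health drops and adds points to the FPS map game mode's score.
; Custom destroy toggles tank mesh collision by remaining health and unpossesses the AI controller at zero health.
; The attack function only prints a debug message, and the event graph is empty.
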(event `self.ReceiveActorBeginOverlap`
  (params (OtherActor :type "Actor Object Reference")))

(fn `CustomDestroy`
  (params (isVisible :type Boolean) (HasCollision :type Boolean))
  (bind _tankmesh (`self.TankMesh`))
  (`parent.CustomDestroy` isVisible HasCollision)
  (if (> (`/Game/FPS/Blueprints/BP_Health_Component.Health` (`self.BP_Health_Component`)) 0.0)
    (`PrimitiveComponent.SetCollisionEnabled` _tankmesh "QueryAndPhysics")
    (else
      (`PrimitiveComponent.SetCollisionEnabled` _tankmesh "NoCollision")
      (`Controller.UnPossess` (`AIBlueprintHelperLibrary.GetAIController` self)))))

(fn `OnAttack`
  (`KismetSystemLibrary.PrintString` "Enemy Attacking"))

(fn `TakeDamage`
  (params (Damage :type "Float (double-precision)"))
  (`parent.TakeDamage` Damage)
  (`self.UpdateScale`)
  (bind _asgm_fpsmap (cast `/Game/FPS/Blueprints/GM_FPSMap` (`GameplayStatics.GetGameMode`)))
  (`/Game/FPS/Blueprints/GM_FPSMap.AddPointsToScore` _asgm_fpsmap (`self.Add Score Points`)))

(fn `UpdateScale`
  (bind _bp_health_component (`self.BP_Health_Component`))
  (bind _output_get (set `self.FullScale` (1.0 1.0 1.0)))
  (`SceneComponent.SetWorldScale3D` (`self.NS_Fire`) (* (`KismetMathLibrary.FClamp` (- 1.0 (/ (`/Game/FPS/Blueprints/BP_Health_Component.Health` _bp_health_component) (`/Game/FPS/Blueprints/BP_Health_Component.MaxHealth` _bp_health_component)))) _output_get)))

(fn `UserConstructionScript`)