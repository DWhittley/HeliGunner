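; BP_Tank is an enemy tank Blueprint whose fire effect grows as it loses health.
; After the parent damage handling, UpdateScale sets NSFire's world scale to the clamped missing-health fraction.
; CustomDestroy extends the parent and sets fire visibility.
; Its constant-true branch always enables mesh collision and sets the fire to the tank mesh scale cached at BeginPlay, leaving the collision-disable path unreachable.
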(event `self.ReceiveBeginPlay`
  (set `self.OriginalScale` (`SceneComponent.K2_GetComponentScale` (`self.TankMesh`))))

(fn `CustomDestroy`
  (params (isVisible :type Boolean) (HasCollision :type Boolean))
  (bind _returnvalue (!= isVisible false))
  (bind _tankmesh (`self.TankMesh`))
  (`parent.CustomDestroy` _returnvalue HasCollision)
  (`SceneComponent.SetVisibility` (`self.NS_Fire`) _returnvalue false)
  (if true
    (`PrimitiveComponent.SetCollisionEnabled` _tankmesh "QueryAndPhysics")
    (`SceneComponent.SetWorldScale3D` (`self.NS_Fire`) (`self.OriginalScale`))
    (else
      (`PrimitiveComponent.SetCollisionEnabled` _tankmesh "NoCollision"))))

(fn `TakeDamage`
  (params (Damage :type "Float (double-precision)"))
  (`parent.TakeDamage` Damage)
  (`self.UpdateScale`))

(fn `UpdateScale`
  (bind _bp_health_component (`self.BP_Health_Component`))
  (bind _output_get (set `self.FulllScale` (1.0 1.0 1.0)))
  (`SceneComponent.SetWorldScale3D` (`self.NS_Fire`) (* (`KismetMathLibrary.FClamp` (- 1.0 (/ (`/Game/FPS/Blueprints/BP_Health_Component.Health` _bp_health_component) (`/Game/FPS/Blueprints/BP_Health_Component.MaxHealth` _bp_health_component)))) _output_get)))

(fn `UserConstructionScript`
  (`parent.UserConstructionScript`))