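; GM_FPSMap is a Blueprint, apparently the FPS map's game mode, that puts up the score HUD and tracks score and high score.
; On BeginPlay it creates the W_PlayerScore widget and adds it to the viewport.
; The AddPointsToScore event adds points to Score and raises HighestScore when the new total exceeds it.
; The destroyed-actor binding never runs, and its handler and TestFunction are empty.
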(event `self.ReceiveBeginPlay`
  (bind _returnvalue (`|CreateWidget` "/Game/FPS/UI/W_PlayerScore.W_PlayerScore_C"))
  (`UserWidget.AddToViewport` _returnvalue 0))

(event `OnDestroyed_Event` :!signature `self.OnDestroyed`
  (params (DestroyedActor :type "Actor Object Reference")))

(event `AddPointsToScore`
  (params (AddScorePoints :type Integer))
  (bind _output_get (set `self.Score` (+ AddScorePoints (`self.Score`))))
  ;[1 1 1] Update High Score
  (`/Engine/EditorBlueprintResources/StandardMacros.CompareInt` _output_get (`self.HighestScore`)
    (:`>`
      (set `self.HighestScore` _output_get))))

(fn `TestFunction`)

(fn `UserConstructionScript`)