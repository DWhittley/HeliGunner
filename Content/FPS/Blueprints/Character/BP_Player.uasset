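; BP_Player is the first-person player character, handling movement, mouse-style look and gun firing.
; On BeginPlay it spawns StartingGun, stores it as EquippedGun and attaches it to GunSpawnPoint at the Equipped_Weapon socket.
; Axis inputs drive movement and look, while held Shoot input passes through a Delay of the gun's FireRate, throttling shots.
; Each shot hands the gun a camera-forward segment scaled by its Range.
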(event `self.ReceiveBeginPlay`
  (bind _returnvalue (`|SpawnActorFromClass` (`self.Starting Gun`) (`KismetMathLibrary.MakeTransform` (0.0 0.0 0.0)) "Undefined" "SelectDefaultAtRuntime" null null))
  (bind _asbp_gun (cast `/Game/FPS/Blueprints/Gun/BP_Gun` _returnvalue))
  (bind _output_get (set `self.EquippedGun` _asbp_gun))
  (`self.K2_AttachToComponent` _output_get (`self.GunSpawnPoint`) "Equipped_Weapon" "KeepRelative" "KeepRelative" "KeepRelative" true))

(event `InputAxis|Move Forward`
  (params (AxisValue :type "Float (single-precision)"))
  ;[1 1 1] Movement
  (`self.AddMovementInput` (`self.GetActorForwardVector`) AxisValue))

(event `InputAxis|Shoot`
  (params (AxisValue :type "Float (single-precision)"))
  (bind _equippedgun (`self.EquippedGun`))
  (bind _camera (`self.Camera`))
  (bind _returnvalue (`SceneComponent.K2_GetComponentLocation` _camera))
  ;[1 1 1] Shooting
  (if (> AxisValue 0.0)
    (`KismetSystemLibrary.Delay` (`/Game/FPS/Blueprints/Gun/BP_Gun.FireRate` _equippedgun))
    (`/Game/FPS/Blueprints/Gun/BP_Gun.Shoot` _equippedgun _returnvalue (+ _returnvalue (* (`SceneComponent.GetForwardVector` _camera) (`/Game/FPS/Blueprints/Gun/BP_Gun.Range` (`self.EquippedGun`)))))))

(event `InputAxis|Move Left`
  (params (AxisValue :type "Float (single-precision)"))
  ;[1 1 1] Movement
  (`self.AddMovementInput` (`self.GetActorRightVector`) AxisValue))

(event `InputAxis|Look Horizontal`
  (params (AxisValue :type "Float (single-precision)"))
  ;[1 1 1] Movement
  (`self.AddControllerYawInput` AxisValue))

(event `InputAxis|Look Vertical`
  (params (AxisValue :type "Float (single-precision)"))
  ;[1 1 1] Movement
  (`self.AddControllerPitchInput` (* AxisValue -1.0)))

(fn `UserConstructionScript`)