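; BP_Helo is a helicopter actor that carries the player along a spline path and ends the game when the run finishes.
; The MoveHelo timeline, rate-scaled by Duration, sets its location and rotation from PathRef's spline.
; Tick pins the player character 500 units above it, and timeline completion shows W_GameOver with the cursor and pauses the game.
; BeginPlay stores the found BP_HeloPath in HeloPathReference, though movement reads PathRef.
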(event `self.ReceiveBeginPlay`
  (bind _returnvalue (`GameplayStatics.GetActorOfClass` "/Game/FPS/Blueprints/HeloPath/BP_HeloPath.BP_HeloPath_C"))
  (set `self.HeloPathReference` _returnvalue)
  (`self.MovingHelo`))

(event `MovingHelo`
  (bind _spline (`/Game/FPS/Blueprints/HeloPath/BP_HeloPath.Spline` (`self.PathRef`)))
  (`TimelineComponent.SetPlayRate` (`self.MoveHelo`) (/ 1.0 (`self.duration`)))
  ;[1 1 1] Platform Movement
  (bind (_direction _alpha) (`Timeline|MoveHelo`)
    (:`Update`
      (bind _returnvalue (`KismetMathLibrary.Lerp` 0.0 (`SplineComponent.GetSplineLength` _spline) _alpha))
      (`self.K2_SetActorTransform` (`KismetMathLibrary.MakeTransform` (`SplineComponent.GetLocationAtDistanceAlongSpline` _spline _returnvalue "World") (`SplineComponent.GetRotationAtDistanceAlongSpline` _spline _returnvalue "World"))))
    (:`Finished`
      ;[1 1 1] At end of run show game over screen
      (bind _returnvalue_2 (`|CreateWidget` "/Game/FPS/UI/Screens/W_GameOver.W_GameOver_C"))
      (`UserWidget.AddToViewport` _returnvalue_2 0)
      (set `PlayerController.bShowMouseCursor` true (`GameplayStatics.GetPlayerController` 0))
      (`GameplayStatics.SetGamePaused` true))))

(event `self.ReceiveTick`
  (params (DeltaSeconds :type "Float (single-precision)"))
  ;[1 1 1] Move player with platform
  (`self.K2_SetActorLocation` (`GameplayStatics.GetPlayerCharacter` 0) (+ (`self.K2_GetActorLocation`) (0.0 0.0 500.0)) false false))

(fn `UserConstructionScript`)